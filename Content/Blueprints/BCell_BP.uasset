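; B cell actor that drifts in a simulated fluid and responds to collisions.
; Construction picks a random mesh from NeutrophilMeshes (despite the B cell name), gives it a random rotation and calls MoveWithFluid on it.
; Tick calls ApplyFluid on the mesh and animates its materials' Translation parameter from time since creation.
; Hit events are forwarded to HandleCollision.
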(event `self.ReceiveBeginPlay`)

(event `self.ReceiveTick`
  (params (DeltaSeconds :type "Float (single-precision)"))
  (bind _staticmesh (`self.StaticMesh`))
  (`FluidDynamics.ApplyFluid` _staticmesh)
  (`MeshComponent.SetScalarParameterValueOnMaterials` _staticmesh "Translation" (* (`self.GetGameTimeSinceCreation`) 0.2)))

(event `self.ReceiveHit`
  (params (MyComp :type "PrimitiveComponent Object Reference") (Other :type "Actor Object Reference") (OtherComp :type "PrimitiveComponent Object Reference") (bSelfMoved :type Boolean) (HitLocation :type "Vector Structure") (HitNormal :type "Vector Structure") (NormalImpulse :type "Vector Structure") (Hit :type "HitResult Structure (by ref)"))
  (`self.HandleCollision` MyComp Other OtherComp NormalImpulse Hit))

(fn `UserConstructionScript`
  (bind _staticmesh (`self.StaticMesh`))
  (bind _neutrophil_meshes (`self.Neutrophil Meshes`))
  (`StaticMeshComponent.SetStaticMesh` (`self.StaticMesh`) (`|GetArrayItem` _neutrophil_meshes (`KismetMathLibrary.RandomInteger` (`KismetArrayLibrary.Array_Length` _neutrophil_meshes))))
  (`FluidDynamics.MoveWithFluid` _staticmesh 0.3)
  (`SceneComponent.K2_SetWorldRotation` _staticmesh (`KismetMathLibrary.MakeRotator` (`KismetMathLibrary.RandomFloatInRange` 0.0 360.0) (`KismetMathLibrary.RandomFloatInRange` 0.0 360.0) (`KismetMathLibrary.RandomFloatInRange` 0.0 360.0)) false false))