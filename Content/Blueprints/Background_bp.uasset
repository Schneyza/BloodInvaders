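; Background actor that endlessly scrolls two blood-stream components along its local X axis.
; Each Tick, it derives both relative X positions from time since creation multiplied by VelocityX, rather than accumulating movement.
; A modulo wraps each position, and a half-period offset staggers the two pieces so they leapfrog as a looping backdrop.
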(event `self.ReceiveTick`
  (params (DeltaSeconds :type "Float (single-precision)"))
  (bind _returnvalue (* (`self.GetGameTimeSinceCreation`) (`self.Velocity X`)))
  (`SceneComponent.K2_SetRelativeLocation` (`self.Background_BloodStream_3`) (`KismetMathLibrary.MakeVector` (+ (mod (+ _returnvalue -6000.0) 12000.0) 4000.0)) false false)
  (`SceneComponent.K2_SetRelativeLocation` (`self.Background_BloodStream_31`) (`KismetMathLibrary.MakeVector` (+ (mod _returnvalue 12000.0) 4000.0)) false false))

(fn `UserConstructionScript`)