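; Cell actor whose Cube mesh reacts to the player every tick, under a graph section labeled Virus.
; Tick turns on the cube's custom depth rendering while the player controller's location is within a fixed range.
; It also rotates the cube to face that location.
; An ApplyFluid call on the cube sits in the graph but never runs.
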(event `self.ReceiveActorBeginOverlap`
  (params (OtherActor :type "Actor Object Reference")))

(event `self.ReceiveTick`
  (params (DeltaSeconds :type "Float (single-precision)"))
  (bind _cube (`self.Cube`))
  (bind _returnvalue (`SceneComponent.K2_GetComponentLocation` (`self.Cube`)))
  (bind _returnvalue_2 (`self.K2_GetActorLocation` (`GameplayStatics.GetPlayerController` 0)))
  (`PrimitiveComponent.SetRenderCustomDepth` _cube (<= (`KismetMathLibrary.VSize` (- _returnvalue_2 _returnvalue)) 1000.0))
  (`SceneComponent.K2_SetWorldRotation` _cube (`KismetMathLibrary.FindLookAtRotation` _returnvalue _returnvalue_2) false false))

(fn `UserConstructionScript`)