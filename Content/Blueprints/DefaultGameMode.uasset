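; Game mode that spawns the cells of an immune-system game: infectable, red blood, macrophage, neutrophil, B cell and T helper.
; Each type has its own spawn event, triggered from outside this graph, that places the actor via GetSpawnPoint.
; GetSpawnPoint picks a random point in SpawnVolume, falling back to the world origin when the volume is invalid.
; New macrophages also get their neutrophil and dendritic messenger timers started.
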(event `self.SpawnInfectableBP`
  ;[1 1 1] Spawn Infectable Cell
  (bind _spawnpoint (`self.GetSpawnPoint`))
  (`|SpawnActorFromClass` "/Game/Blueprints/Cell_bp.Cell_bp_C" _spawnpoint "AdjustIfPossibleButAlwaysSpawn" "OverrideRootScale" null null))

(event `self.SpawnBloodCellBP`
  ;[1 1 1] Spawn Red Blood Cell
  (bind _spawnpoint (`self.GetSpawnPoint`))
  (`|SpawnActorFromClass` "/Game/Blueprints/RedBloodCellBP.RedBloodCellBP_C" _spawnpoint "AdjustIfPossibleButAlwaysSpawn" "OverrideRootScale" null null))

(event `self.SpawnMacrophageBP`
  ;[1 1 1] Spawn Macrophage
  (bind _spawnpoint (`self.GetSpawnPoint`))
  (bind _returnvalue (`|SpawnActorFromClass` "/Game/Blueprints/MacrophageBP.MacrophageBP_C" _spawnpoint "AdjustIfPossibleButAlwaysSpawn" "OverrideRootScale" null null))
  (`/Game/Blueprints/MacrophageBP.StartNeutrophilMessengerTimer` _returnvalue)
  (`/Game/Blueprints/MacrophageBP.StartDendriticMessengerTimer` _returnvalue))

(event `self.SpawnNeutrophilBP`
  ;[1 1 1] Spawn Neutrophil
  (bind _spawnpoint (`self.GetSpawnPoint`))
  (`|SpawnActorFromClass` "/Game/Blueprints/neutrophil_bp.neutrophil_bp_C" _spawnpoint "AdjustIfPossibleButAlwaysSpawn" "OverrideRootScale" null null))

(event `self.SpawnBCellBP`
  ;[1 1 1] Spawn BCell
  (bind _spawnpoint (`self.GetSpawnPoint`))
  (`|SpawnActorFromClass` "/Game/Blueprints/BCell_BP.BCell_BP_C" _spawnpoint "Undefined" "OverrideRootScale" null null))

(event `self.SpawnTHelperBP`
  ;[1 1 1] Spawn THelper
  (bind _spawnpoint (`self.GetSpawnPoint`))
  (`|SpawnActorFromClass` "/Game/Blueprints/THelper_BP.THelper_BP_C" _spawnpoint "Undefined" "OverrideRootScale" null null))

(fn `GetSpawnPoint`
  (returns (SpawnPoint :type "Transform Structure"))
  (bind _spawnvolume (`self.SpawnVolume`))
  (if (`KismetSystemLibrary.IsValid` _spawnvolume)
    (return (`KismetMathLibrary.MakeTransform` (`SpawnVolume.GetRandomPointInVolume` _spawnvolume)))
    (else
      (return (`KismetMathLibrary.MakeTransform` (0.0 0.0 0.0))))))

(fn `UserConstructionScript`)