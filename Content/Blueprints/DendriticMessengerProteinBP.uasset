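; Dendritic messenger protein actor for Blood Invaders that, shortly after spawning, signals the game mode to raise immune cell spawn chances.
; Construction gives Protein1 a random mesh, material and rotation for visual variety.
; BeginPlay sets two equal-delay timers by function name, one for B cells and one for T helpers, each calling the game mode then destroying the actor.
; Hit events pass to HandleCollision, while an ApplyFluid call is left unwired.
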(event `self.ReceiveBeginPlay`
  (`KismetSystemLibrary.K2_SetTimer` null "IncreaseBCellSpawnChance" 5.0)
  (`KismetSystemLibrary.K2_SetTimer` null "IncreaseTHelperSpawnChance" 5.0))

(event `self.ReceiveTick`
  (params (DeltaSeconds :type "Float (single-precision)")))

(event `self.ReceiveHit`
  (params (MyComp :type "PrimitiveComponent Object Reference") (Other :type "Actor Object Reference") (OtherComp :type "PrimitiveComponent Object Reference") (bSelfMoved :type Boolean) (HitLocation :type "Vector Structure") (HitNormal :type "Vector Structure") (NormalImpulse :type "Vector Structure") (Hit :type "HitResult Structure (by ref)"))
  (`self.HandleCollision` MyComp Other OtherComp NormalImpulse Hit))

(event `self.ReceiveDestroyed`)

(fn `IncreaseBCellSpawnChance`
  (bind _asblood_invaders_game_mode (cast `BloodInvadersGameMode` (`GameplayStatics.GetGameMode`)))
  (`BloodInvadersGameMode.IncreaseBCellSpawnChance` _asblood_invaders_game_mode)
  (`self.K2_DestroyActor`))

(fn `IncreaseTHelperSpawnChance`
  (bind _asblood_invaders_game_mode (cast `BloodInvadersGameMode` (`GameplayStatics.GetGameMode`)))
  (`BloodInvadersGameMode.IncreaseTHelperSpawnChance` _asblood_invaders_game_mode)
  (`self.K2_DestroyActor`))

(fn `UserConstructionScript`
  (bind _protein1 (`self.Protein1`))
  (bind _protein_meshes (`self.Protein Meshes`))
  (bind _protein_materials (`self.Protein Materials`))
  (set `self.Mesh` _protein1)
  (`StaticMeshComponent.SetStaticMesh` _protein1 (`|GetArrayItem` _protein_meshes (`KismetMathLibrary.RandomInteger` (`KismetArrayLibrary.Array_Length` _protein_meshes))))
  (`PrimitiveComponent.SetMaterial` _protein1 0 (`|GetArrayItem` _protein_materials (`KismetMathLibrary.RandomInteger` (`KismetArrayLibrary.Array_Length` _protein_materials))))
  (`SceneComponent.K2_SetWorldRotation` _protein1 (`KismetMathLibrary.MakeRotator` (`KismetMathLibrary.RandomFloatInRange` 0.0 360.0) (`KismetMathLibrary.RandomFloatInRange` 0.0 360.0) (`KismetMathLibrary.RandomFloatInRange` 0.0 360.0)) false false))