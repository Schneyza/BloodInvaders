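; B cell enemy that periodically fires a ring of projectiles outward around itself.
; A looping timer started on BeginPlay spawns evenly spaced BCellProjectile_BP actors on a world-horizontal circle, optionally staggered into a sweep by DelayedFire.
; Construction randomizes the mesh rotation and calls MoveWithFluid on it, while hits pass to HandleCollision.
; The ApplyFluid call in the event graph is disconnected.
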(event `ShootEvent`
  (bind _projectilespawnradius (`self.ProjectileSpawnRadius`))
  (bind _output_get (set `self.Index` 0.0))
  (set `self.ZRotation` 90.0)
  (if (< _output_get 360.0) :!label _label
    (`|SpawnActorFromClass` "/Game/Blueprints/Projectiles/BCellProjectile_BP.BCellProjectile_BP_C" (`KismetMathLibrary.MakeTransform` (+ (`KismetMathLibrary.MakeVector` (* (`KismetMathLibrary.DegSin` _output_get) _projectilespawnradius) (* _projectilespawnradius (`KismetMathLibrary.DegCos` _output_get))) (`SceneComponent.K2_GetComponentLocation` (`self.StaticMesh`))) (`KismetMathLibrary.MakeRotator` 0.0 0.0 (`self.ZRotation`))) "AdjustIfPossibleButAlwaysSpawn" "OverrideRootScale" null null)
    (if (`self.DelayedFire`)
      (`KismetSystemLibrary.Delay` 0.05))
    (set `self.Index` (+ (`self.Index`) 30.0))
    (set `self.ZRotation` (- (`self.ZRotation`) 30.0))
    (goto _label)))

(event `self.ReceiveBeginPlay`
  (`KismetSystemLibrary.K2_SetTimerDelegate` (delegate `ShootEvent`) 2.0 true))

(event `self.ReceiveTick`
  (params (DeltaSeconds :type "Float (single-precision)")))

(event `self.ReceiveHit`
  (params (MyComp :type "PrimitiveComponent Object Reference") (Other :type "Actor Object Reference") (OtherComp :type "PrimitiveComponent Object Reference") (bSelfMoved :type Boolean) (HitLocation :type "Vector Structure") (HitNormal :type "Vector Structure") (NormalImpulse :type "Vector Structure") (Hit :type "HitResult Structure (by ref)"))
  (`self.HandleCollision` MyComp Other OtherComp NormalImpulse Hit))

(fn `UserConstructionScript`
  (bind _staticmesh (`self.StaticMesh`))
  (`FluidDynamics.MoveWithFluid` _staticmesh 0.3)
  (`SceneComponent.K2_SetWorldRotation` _staticmesh (`KismetMathLibrary.MakeRotator` (`KismetMathLibrary.RandomFloatInRange` 0.0 360.0) (`KismetMathLibrary.RandomFloatInRange` 0.0 360.0) (`KismetMathLibrary.RandomFloatInRange` 0.0 360.0)) false false))