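; Cell actor that the player virus can infect, drifting via fluid forces until infected.
; Tick distance checks toggle a custom-depth highlight, hint text and actor input near the player, replacing the unused trigger-overlap logic.
; The ability key asks the player to infect it; success increments score, enlarges the cell and disables its physics and collision.
; Projectiles that hit it are destroyed, and EndInfect destroys the cell.
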(event `self.ReceiveTick`
  (params (DeltaSeconds :type "Float (single-precision)"))
  (`|ExecutionSequence`
    (:`then_0`
      ;[1 1 1] Fluid if not infected
      (if (not (`self.Infected`))
        (`FluidDynamics.ApplyFluid` (`self.CellMesh`))))
    (:`then_1`
      ;[1 1 1] Highlight
      (`/Engine/EditorBlueprintResources/StandardMacros.CompareFloat` (`KismetMathLibrary.VSize` (- (`SceneComponent.K2_GetComponentLocation` (`self.CellMesh`)) (`self.K2_GetActorLocation` (`GameplayStatics.GetPlayerPawn` 0)))) 500.0
        (:`>`
          (`self.HighlightOff`))
        (:`==`
          (`self.HighlightOn` :!label _label)
          (`self.UpdateHintTextLocation`))
        (:`<`
          (goto _label))))))

(event `InputAction|Ability1_P1`
  (params (Key :type "Key Structure"))
  (:`Pressed`
    (bind _asplayer_virus_bp (cast `/Game/Blueprints/Player/PlayerVirus_BP` (`GameplayStatics.GetPlayerPawn` 0)))
    (bind _returnvalue (`Virus.infect` _asplayer_virus_bp self (`self.CellMesh`)))
    (set `self.ShowHint` false)
    (`self.HighlightOff`)
    (if _returnvalue
      (`self.Infect`)
      (`/Game/Blueprints/FL_Score.Increment Score Entry` "NewEnumerator0"))))

(event `self.TriggerVolumeUnused.OnComponentBeginOverlap`
  (params (OverlappedComponent :type "PrimitiveComponent Object Reference") (OtherActor :type "Actor Object Reference") (OtherComp :type "PrimitiveComponent Object Reference") (OtherBodyIndex :type Integer) (bFromSweep :type Boolean) (SweepResult :type "HitResult Structure (by ref)")))

(event `self.TriggerVolumeUnused.OnComponentEndOverlap`
  (params (OverlappedComponent :type "PrimitiveComponent Object Reference") (OtherActor :type "Actor Object Reference") (OtherComp :type "PrimitiveComponent Object Reference") (OtherBodyIndex :type Integer)))

(event `self.ReceiveHit`
  (params (MyComp :type "PrimitiveComponent Object Reference") (Other :type "Actor Object Reference") (OtherComp :type "PrimitiveComponent Object Reference") (bSelfMoved :type Boolean) (HitLocation :type "Vector Structure") (HitNormal :type "Vector Structure") (NormalImpulse :type "Vector Structure") (Hit :type "HitResult Structure (by ref)"))
  (bind _asprojectile (cast `Projectile` Other))
  (`self.K2_DestroyActor` _asprojectile))

(fn `EndInfect`
  (`self.K2_DestroyActor`))

(fn `HighlightOff`
  (if (`self.Highlighted`)
    (set `self.Highlighted` false)
    (`self.DisableInput` (`GameplayStatics.GetPlayerController` 0))
    (`PrimitiveComponent.SetRenderCustomDepth` (`self.CellMesh`) false)
    (`SceneComponent.SetVisibility` (`self.HintText`) false false)))

(fn `HighlightOn`
  (if (not (`self.Highlighted`))
    (set `self.Highlighted` true)
    (`PrimitiveComponent.SetRenderCustomDepth` (`self.CellMesh`) true)
    (`self.EnableInput` (`GameplayStatics.GetPlayerController` 0))
    (if (`self.ShowHint`)
      (`SceneComponent.SetVisibility` (`self.HintText`) true false))))

(fn `Infect`
  (bind _cellmesh (`self.CellMesh`))
  (set `self.Infected` true)
  (`SceneComponent.SetWorldScale3D` (`self.DefaultSceneRoot`) (1.2 1.2 1.2))
  (`PrimitiveComponent.SetSimulatePhysics` _cellmesh false)
  (`PrimitiveComponent.SetCollisionEnabled` _cellmesh "NoCollision"))

(fn `UpdateHintTextLocation`
  (bind (_returnvalue_x _returnvalue_y) (`KismetMathLibrary.BreakVector` (`SceneComponent.K2_GetComponentLocation` (`self.CellMesh`))))
  (`SceneComponent.K2_SetWorldLocation` (`self.HintText`) (`KismetMathLibrary.MakeVector` _returnvalue_x _returnvalue_y 200.0) false false))

(fn `UserConstructionScript`)