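; Macrophage enemy for Blood Invaders that hunts players and can release immune messenger proteins.
; Each tick it faces the nearest visible player, drifts toward them only while they are at lower X, applies fluid force, and wobbles via phase-shifted sine morph targets.
; Hits go to HandleCollision.
; Self-rearming timer functions spawn Neutrophil and Dendritic messengers at an offset using GameMode intervals and chances; the Dendritic starter polls until the GameMode enables it.
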(event `self.ReceiveBeginPlay`)

(event `self.ReceiveTick`
  (params (DeltaSeconds :type "Float (single-precision)"))
  (bind _returnvalue (`self.GetGameTimeSinceCreation`))
  (bind _sphere (`self.Sphere`))
  (bind _macrophage_icosphere (`self.Macrophage_Icosphere`))
  (bind _returnvalue_2 (`SceneComponent.K2_GetComponentLocation` _sphere))
  (bind _returnvalue_3 (`self.K2_GetActorLocation` (`|GetArrayItem` (`self.Players`) (`self.ClosestPlayerIndex`))))
  (bind _returnvalue_4 (`KismetMathLibrary.FindLookAtRotation` _returnvalue_2 _returnvalue_3))
  (bind _outactors (`GameplayStatics.GetAllActorsOfClass` "/Script/BloodInvaders.BloodInvadersPlayer"))
  (set `self.Players` _outactors)
  ;[1 1 1] Set Variables Related to Closest Player
  (set `self.ClosestPlayerDistance` 999999999999.0)
  (for (_array_element _array_index) (`self.Players`)
    (if (not (`Actor.bHidden` _array_element))
      (bind _returnvalue_5 (`self.GetDistanceTo` _array_element))
      (`/Engine/EditorBlueprintResources/StandardMacros.CompareFloat` _returnvalue_5 (`self.ClosestPlayerDistance`)
        (:`<`
          (set `self.ClosestPlayerDistance` _returnvalue_5)
          (set `self.ClosestPlayerIndex` _array_index)))))
  (if (> (.x _returnvalue_2) (.x _returnvalue_3))
    ;[1 1 1] Follow the Closest Player
    (`SceneComponent.K2_SetWorldLocationAndRotation` _sphere (`KismetMathLibrary.VInterpTo` _returnvalue_2 _returnvalue_3 (`GameplayStatics.GetWorldDeltaSeconds`) 0.1) _returnvalue_4 false false)
    (else
      (`SceneComponent.K2_SetWorldRotation` (`self.Sphere`) _returnvalue_4 false false)))
  (`FluidDynamics.ApplyFluidForce` (`self.Sphere`))
  (`SkeletalMeshComponent.SetMorphTarget` _macrophage_icosphere "Deform1" (`KismetMathLibrary.Sin` _returnvalue) true)
  (`SkeletalMeshComponent.SetMorphTarget` _macrophage_icosphere "Deform2" (`KismetMathLibrary.Sin` (+ _returnvalue 1.57)) true))

(event `self.ReceiveHit`
  (params (MyComp :type "PrimitiveComponent Object Reference") (Other :type "Actor Object Reference") (OtherComp :type "PrimitiveComponent Object Reference") (bSelfMoved :type Boolean) (HitLocation :type "Vector Structure") (HitNormal :type "Vector Structure") (NormalImpulse :type "Vector Structure") (Hit :type "HitResult Structure (by ref)"))
  (`self.HandleCollision` MyComp Other OtherComp NormalImpulse Hit))

(fn `SpawnDendriticMessenger`
  (bind _asblood_invaders_game_mode (cast `BloodInvadersGameMode` (`GameplayStatics.GetGameMode`)))
  (if (< (`KismetMathLibrary.RandomFloatInRange` 0.0 1.0) (`BloodInvadersGameMode.DendriticMessengerSpawnChance` _asblood_invaders_game_mode))
    (`|SpawnActorFromClass` "/Game/Blueprints/Proteins/DendriticMessengerProteinBP.DendriticMessengerProteinBP_C" (`KismetMathLibrary.MakeTransform` (`KismetMathLibrary.TransformLocation` (`KismetMathLibrary.MakeTransform` (`self.ProteinSpawnXOffset`)) (`SceneComponent.K2_GetComponentLocation` (`self.Sphere`)))) "AdjustIfPossibleButAlwaysSpawn" "OverrideRootScale" null null))
  (bind _dendriticmessengerspawninterval (`BloodInvadersGameMode.DendriticMessengerSpawnInterval` _asblood_invaders_game_mode))
  (if (> _dendriticmessengerspawninterval 0.0)
    (`KismetSystemLibrary.K2_SetTimer` null "SpawnDendriticMessenger" _dendriticmessengerspawninterval)))

(fn `SpawnNeutrophilMessenger`
  (bind _asblood_invaders_game_mode (cast `BloodInvadersGameMode` (`GameplayStatics.GetGameMode`)))
  (if (< (`KismetMathLibrary.RandomFloatInRange` 0.0 1.0) (`BloodInvadersGameMode.NeutrophilMessengerSpawnChance` _asblood_invaders_game_mode))
    (`|SpawnActorFromClass` "/Game/Blueprints/Proteins/NeutrophilMessengerProtein.NeutrophilMessengerProtein_C" (`KismetMathLibrary.MakeTransform` (`KismetMathLibrary.TransformLocation` (`KismetMathLibrary.MakeTransform` (`self.ProteinSpawnXOffset`)) (`SceneComponent.K2_GetComponentLocation` (`self.Sphere`)))) "AdjustIfPossibleButAlwaysSpawn" "OverrideRootScale" null null))
  (bind _neutrophilmessengerspawninterval (`BloodInvadersGameMode.NeutrophilMessengerSpawnInterval` _asblood_invaders_game_mode))
  (if (> _neutrophilmessengerspawninterval 0.0)
    (`KismetSystemLibrary.K2_SetTimer` null "SpawnNeutrophilMessenger" _neutrophilmessengerspawninterval)))

(fn `StartDendriticMessengerTimer`
  (bind _asblood_invaders_game_mode (cast `BloodInvadersGameMode` (`GameplayStatics.GetGameMode`)))
  (if (`BloodInvadersGameMode.DendriticMessengerSpawnStarted` _asblood_invaders_game_mode)
    (`KismetSystemLibrary.K2_SetTimer` null "SpawnDendriticMessenger" (`BloodInvadersGameMode.DendriticMessengerSpawnInterval` _asblood_invaders_game_mode))
    (else
      (`KismetSystemLibrary.K2_SetTimer` null "StartDendriticMessengerTimer" 5.0))))

(fn `StartNeutrophilMessengerTimer`
  (bind _asblood_invaders_game_mode (cast `BloodInvadersGameMode` (`GameplayStatics.GetGameMode`)))
  (`KismetSystemLibrary.K2_SetTimer` null "SpawnNeutrophilMessenger" (`BloodInvadersGameMode.NeutrophilMessengerSpawnInterval` _asblood_invaders_game_mode)))

(fn `UserConstructionScript`)