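; RBCBacterium is an enemy bacterium built around a RedBloodCell component, with its own health and damage values.
; Its construction script sets max and current health from StartHealth and damage from BactDamage.
; Each tick it applies fluid to the cell, and hits are passed to HandleCollision.
; When destroyed, it spawns an explosion effect and an enlarged ProteinBacterium at the cell's location.
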(event `self.ReceiveTick`
  (params (DeltaSeconds :type "Float (single-precision)"))
  (`FluidDynamics.ApplyFluid` (`self.Red_Blood_Cell`)))

(event `self.ReceiveHit`
  (params (MyComp :type "PrimitiveComponent Object Reference") (Other :type "Actor Object Reference") (OtherComp :type "PrimitiveComponent Object Reference") (bSelfMoved :type Boolean) (HitLocation :type "Vector Structure") (HitNormal :type "Vector Structure") (NormalImpulse :type "Vector Structure") (Hit :type "HitResult Structure (by ref)"))
  (`self.HandleCollision` MyComp Other OtherComp NormalImpulse Hit))

(event `self.ReceiveDestroyed`
  (bind _returnvalue (`SceneComponent.K2_GetComponentLocation` (`self.Red_Blood_Cell`)))
  (`GameplayStatics.SpawnEmitterAtLocation` "/Game/StarterContent/Particles/P_Explosion.P_Explosion" _returnvalue (struct) (3.0 3.0 3.0))
  (`|SpawnActorFromClass` "/Game/Blueprints/Proteins/ProteinBacterium.ProteinBacterium_C" (`KismetMathLibrary.MakeTransform` _returnvalue (struct) (5.0 5.0 5.0)) "AlwaysSpawn" "OverrideRootScale" null null))

(fn `UserConstructionScript`
  (bind _output_get (set `self.MaxHealth` (`self.StartHealth`)))
  (set `self.CurrentHealth` _output_get)
  (set `self.BacteriumDamage` (`self.BactDamage`)))