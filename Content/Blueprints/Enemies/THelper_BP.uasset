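; THelper_BP is an enemy that powers up any MasterEnemy it hits, alongside its general collision handling.
; Construction initializes health and bacterium damage and gives the mesh a random rotation.
; Each tick applies fluid behavior to the mesh.
; A Flash event sets a white vector parameter, though its name is None, then restores the cached materials after a brief delay.
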(event `self.ReceiveBeginPlay`)

(event `self.ReceiveTick`
  (params (DeltaSeconds :type "Float (single-precision)"))
  (`FluidDynamics.ApplyFluid` (`self.StaticMesh`)))

(event `self.ReceiveHit`
  (params (MyComp :type "PrimitiveComponent Object Reference") (Other :type "Actor Object Reference") (OtherComp :type "PrimitiveComponent Object Reference") (bSelfMoved :type Boolean) (HitLocation :type "Vector Structure") (HitNormal :type "Vector Structure") (NormalImpulse :type "Vector Structure") (Hit :type "HitResult Structure (by ref)"))
  (`self.HandleCollision` MyComp Other OtherComp NormalImpulse Hit)
  (bind _asmaster_enemy (cast `MasterEnemy` Other))
  (`self.PowerUp` _asmaster_enemy))

(event `self.Flash`
  (bind _staticmesh (`self.StaticMesh`))
  (`/Engine/EditorBlueprintResources/StandardMacros.IsValid` _staticmesh
    (:`Is Valid`
      (bind _output_get (set `self.Materials` (`MeshComponent.GetMaterials` _staticmesh)))
      (`MeshComponent.SetVectorParameterValueOnMaterials` (`self.StaticMesh`) "None" (1.0 1.0 1.0))
      (`KismetSystemLibrary.Delay` 0.05)
      (for (_array_element _array_index) _output_get
        (`PrimitiveComponent.SetMaterial` (`self.StaticMesh`) _array_index _array_element)))))

(fn `UserConstructionScript`
  (bind _output_get (set `self.MaxHealth` (`self.StartHealth`)))
  (set `self.CurrentHealth` _output_get)
  (set `self.BacteriumDamage` (`self.BactDamage`))
  (`SceneComponent.K2_SetWorldRotation` (`self.StaticMesh`) (`KismetMathLibrary.MakeRotator` (`KismetMathLibrary.RandomFloatInRange` 0.0 360.0) (`KismetMathLibrary.RandomFloatInRange` 0.0 360.0) (`KismetMathLibrary.RandomFloatInRange` 0.0 360.0)) false false))