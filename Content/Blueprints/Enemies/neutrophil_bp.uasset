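; Neutrophil enemy that drifts with the fluid, morphs over time and adds to a score entry on death.
; Construction applies fluid motion, randomizes rotation and initializes health and bacterium damage.
; Tick drives morph targets from lifetime and applies fluid to the mesh, while hits pass to HandleCollision.
; Power-ups add health, and Flash sets a white material parameter briefly before reassigning the saved materials.
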(event `self.OnDeath`
  (`/Game/Blueprints/FL_Score.Increment Score Entry` "NewEnumerator7"))

(event `self.ReceiveTick`
  (params (DeltaSeconds :type "Float (single-precision)"))
  (`self.UpdateMorph`))

(event `UpdateMorph`
  (`/Game/Models/MacrophageNew/MorphLib.MorphTarget` (`self.Neutrophil`) (* (`self.GetGameTimeSinceCreation`) 0.5) (`self.morphNames`))
  (`FluidDynamics.ApplyFluid` (`self.Neutrophil`)))

(event `self.ReceiveHit`
  (params (MyComp :type "PrimitiveComponent Object Reference") (Other :type "Actor Object Reference") (OtherComp :type "PrimitiveComponent Object Reference") (bSelfMoved :type Boolean) (HitLocation :type "Vector Structure") (HitNormal :type "Vector Structure") (NormalImpulse :type "Vector Structure") (Hit :type "HitResult Structure (by ref)"))
  (`self.HandleCollision` MyComp Other OtherComp NormalImpulse Hit))

(event `self.PowerUpEvent`
  (set `self.CurrentHealth` (+ (`self.CurrentHealth`) (`self.PowerUpHealthBonus`))))

(event `self.Flash`
  (bind _neutrophil (`self.Neutrophil`))
  (`/Engine/EditorBlueprintResources/StandardMacros.IsValid` _neutrophil
    (:`Is Valid`
      (bind _output_get (set `self.Materials` (`MeshComponent.GetMaterials` _neutrophil)))
      (`MeshComponent.SetVectorParameterValueOnMaterials` (`self.Neutrophil`) "None" (1.0 1.0 1.0))
      (`KismetSystemLibrary.Delay` 0.05)
      (for (_array_element _array_index) _output_get
        (`PrimitiveComponent.SetMaterial` (`self.Neutrophil`) _array_index _array_element)))))

(fn `UserConstructionScript`
  (`FluidDynamics.MoveWithFluid` (`self.Neutrophil`) 0.3)
  (`SceneComponent.K2_SetWorldRotation` (`self.Neutrophil`) (`KismetMathLibrary.MakeRotator` (`KismetMathLibrary.RandomFloatInRange` 0.0 360.0) (`KismetMathLibrary.RandomFloatInRange` 0.0 360.0) (`KismetMathLibrary.RandomFloatInRange` 0.0 360.0)) false true)
  (bind _output_get (set `self.MaxHealth` (`self.StartHealth`)))
  (set `self.CurrentHealth` _output_get)
  (set `self.BacteriumDamage` (`self.BactDamage`)))