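; FL_Score is a Blueprint function library that gives access to the game's score actor.
; GetScore finds the first Score_BP actor in the level with GetAllActorsOfClass and reports whether one exists.
; IncrementScoreEntry uses that lookup to call IncrementEntry on the score actor, doing nothing when none is present.
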(fn `Get Score`
  (returns (`Return Value` :type "/Game/Blueprints/Score_BP Object Reference") (Success :type Boolean))
  (bind _outactors (`GameplayStatics.GetAllActorsOfClass` null "/Game/Blueprints/Score_BP.Score_BP_C"))
  (if (>= (`KismetArrayLibrary.Array_Length` _outactors) 1)
    (return (`|GetArrayItem` _outactors) true)
    (else
      (return null false))))

(fn `Increment Score Entry`
  (params (Entry :type "/Game/Blueprints/EScoreEntry Enum" :default "NewEnumerator4"))
  (bind (_return_value _success) (`self.Get Score` null))
  (if _success
    (`/Game/Blueprints/Score_BP.Increment Entry` _return_value Entry)))