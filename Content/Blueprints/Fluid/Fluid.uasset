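; Fluid Blueprint that configures and animates a turbulent fluid field.
; The construction script passes its interaction strength, turbulence scale and amplitude, and linear velocity variables to their setters.
; Each tick scrolls the field by setting its coordinate offset to FieldAnimation multiplied by the time since the actor's creation.
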(event `self.ReceiveTick`
  (params (DeltaSeconds :type "Float (single-precision)"))
  (`FluidDynamics.setCoordinateOffset` (* (`self.Field animation`) (`self.GetGameTimeSinceCreation`))))

(fn `UserConstructionScript`
  (`FluidDynamics.setInteractionStrength` (`self.Interaction Strength`))
  (`FluidDynamics.setTurbulenceScale` (`self.Turbulence Scale`))
  (`FluidDynamics.setTurbulenceAmplitude` (`self.Turbulence amplitude`))
  (`FluidDynamics.setLinearVelocity` (`self.Linear Velocity`)))