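; FluidIndicator is an actor that visualizes a 2D fluid velocity field as a grid of needle meshes.
; The construction script spawns a CountX by CountY grid of static mesh components around the actor, spaced by Distance, and stores them in Needles.
; Each Tick samples fluid velocity at every needle's world location, rotating it along the flow and scaling it by speed and grid spacing.
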(event `self.ReceiveTick`
  (params (DeltaSeconds :type "Float (single-precision)"))
  (for _array_element (`self.Needles`)
    (bind _returnvalue (`FluidDynamics.getFluidVelocity2D` (`SceneComponent.K2_GetComponentLocation` _array_element)))
    (`SceneComponent.K2_SetWorldRotation` _array_element (`KismetMathLibrary.FindLookAtRotation` (`KismetMathLibrary.MakeVector` 0.0) _returnvalue) false false)
    (`SceneComponent.SetWorldScale3D` _array_element (* (0.8 0.2 0.1) (* (`KismetMathLibrary.VSize` _returnvalue) (* (`self.Distance`) 4e-05))))))

(fn `UserConstructionScript`
  (bind _count_x (`self.Count X`))
  (bind _count_y (`self.Count Y`))
  (bind _distance (`self.Distance`))
  (for _index (range 1 (+ _count_x 1))
    (for _index_2 (range 1 (+ _count_y 1))
      (bind _returnvalue (`AddComponent|NODE_AddStaticMeshComponent-0` :`RelativeTransform` (`KismetMathLibrary.Conv_VectorToTransform` (`KismetMathLibrary.MakeVector` (* (- (`KismetMathLibrary.Conv_IntToDouble` _index) (* (`KismetMathLibrary.Conv_IntToDouble` _count_x) 0.5)) _distance) (* (- (`KismetMathLibrary.Conv_IntToDouble` _index_2) (* (`KismetMathLibrary.Conv_IntToDouble` _count_y) 0.5)) _distance) 25.0))))
      (`KismetArrayLibrary.Array_Add` (`self.Needles`) _returnvalue))))