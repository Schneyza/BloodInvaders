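; FluidNeedle is an actor that visualizes the 2D fluid velocity at its location as a needle.
; Each tick it samples GetFluidVelocity2D at the Cube component's world position and rotates the Cube to point along that velocity.
; The Cube's elongated scale is multiplied by the velocity magnitude and a Size variable, so the needle grows with flow speed.
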(event `self.ReceiveTick`
  (params (DeltaSeconds :type "Float (single-precision)"))
  (bind _cube (`self.Cube`))
  (bind _returnvalue (`FluidDynamics.getFluidVelocity2D` (`SceneComponent.K2_GetComponentLocation` (`self.Cube`))))
  (`SceneComponent.K2_SetWorldRotation` _cube (`KismetMathLibrary.FindLookAtRotation` (`KismetMathLibrary.MakeVector` 0.0) _returnvalue) false false)
  (`SceneComponent.SetWorldScale3D` _cube (* (0.8 0.2 0.1) (* (`KismetMathLibrary.VSize` _returnvalue) (`self.Size`)))))

(fn `UserConstructionScript`)