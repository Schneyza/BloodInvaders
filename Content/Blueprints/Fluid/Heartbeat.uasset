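; Heartbeat actor that runs an endless, timed heartbeat cycle from BeginPlay, pairing a 2D sound with pulses of linear velocity along X.
; Each cycle sets a gentle forward velocity, then a sharp reverse surge that eases off and settles to zero before repeating.
; Shortly after each sound, it calls StartBeat on its FluidPressureWave child actor.
; The loop uses chained Delays rather than Tick or a timer.
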(event `self.ReceiveBeginPlay`
  (`self.Start Heartbeat`))

(event `Start Heartbeat`
  (`GameplayStatics.PlaySound2D` "/Game/Audio/Heartbeat.Heartbeat" :!label _label)
  (`FluidDynamics.setLinearVelocity` (200.0 0.0 0.0))
  (`KismetSystemLibrary.Delay` 0.2)
  (bind _asfluid_pressure_wave (cast `/Game/Blueprints/FluidPressureWave` (`ChildActorComponent.ChildActor` (`self.FluidPressureWave`))))
  (`/Game/Blueprints/FluidPressureWave.StartBeat` _asfluid_pressure_wave)
  (`KismetSystemLibrary.Delay` 0.3)
  (`FluidDynamics.setLinearVelocity` (-2000.0 0.0 0.0))
  (`KismetSystemLibrary.Delay` 0.2)
  (`FluidDynamics.setLinearVelocity` (-200.0 0.0 0.0))
  (`KismetSystemLibrary.Delay` 1.5)
  (`FluidDynamics.setLinearVelocity` (0.0 0.0 0.0))
  (`KismetSystemLibrary.Delay` 1.0)
  (goto _label))

(fn `UserConstructionScript`)