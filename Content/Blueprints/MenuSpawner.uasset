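; MenuSpawner actor that keeps spawning random actors around itself, by its name for a menu scene.
; A looping half-second timer set on BeginPlay calls Spawn, which picks a class from the Types array.
; The random index range includes the array length, so it can land one past the end.
; RandomTransform is meant to randomize position and rotation around the root, but its MakeTransform node appears as unused.
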(event `self.ReceiveBeginPlay`
  (`KismetSystemLibrary.K2_SetTimer` null "Spawn" 0.5 true))

(event `self.ReceiveActorBeginOverlap`
  (params (OtherActor :type "Actor Object Reference")))

(event `self.ReceiveTick`
  (params (DeltaSeconds :type "Float (single-precision)")))

(event `Spawn`
  (bind _types (`self.Types`))
  ;[1 1 1] Create new child
  (`|SpawnActorFromClass` (`|GetArrayItem` _types (`KismetMathLibrary.RandomIntegerInRange` 0 (`KismetArrayLibrary.Array_Length` _types))) (`.Transform` (`self.Random transform` 100.0 (`SceneComponent.K2_GetComponentLocation` (`self.DefaultSceneRoot`)))) "Undefined" "OverrideRootScale" null null))

(fn `UserConstructionScript`)