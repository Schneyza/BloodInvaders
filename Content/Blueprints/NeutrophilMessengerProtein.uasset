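; NeutrophilMessengerProtein is a short-lived messenger protein actor that raises the chance of neutrophils spawning in Blood Invaders.
; The construction script gives the Protein1 component a random rotation on all three axes.
; A five-second timer from BeginPlay tells BloodInvadersGameMode to increase the spawn chance, then destroys the actor.
; Hit events pass to HandleCollision, while an ApplyFluid call is left unwired.
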(event `self.ReceiveBeginPlay`
  (`KismetSystemLibrary.K2_SetTimer` null "IncreaseNeutrophilSpawnChance" 5.0))

(event `self.ReceiveTick`
  (params (DeltaSeconds :type "Float (single-precision)")))

(event `self.ReceiveHit`
  (params (MyComp :type "PrimitiveComponent Object Reference") (Other :type "Actor Object Reference") (OtherComp :type "PrimitiveComponent Object Reference") (bSelfMoved :type Boolean) (HitLocation :type "Vector Structure") (HitNormal :type "Vector Structure") (NormalImpulse :type "Vector Structure") (Hit :type "HitResult Structure (by ref)"))
  (`self.HandleCollision` MyComp Other OtherComp NormalImpulse Hit))

(event `self.ReceiveDestroyed`)

(fn `IncreaseNeutrophilSpawnChance`
  (bind _asblood_invaders_game_mode (cast `BloodInvadersGameMode` (`GameplayStatics.GetGameMode`)))
  (`BloodInvadersGameMode.IncreaseNeutrophilSpawnChance` _asblood_invaders_game_mode)
  (`self.K2_DestroyActor`))

(fn `UserConstructionScript`
  (`SceneComponent.K2_SetWorldRotation` (`self.Protein1`) (`KismetMathLibrary.MakeRotator` (`KismetMathLibrary.RandomFloatInRange` 0.0 360.0) (`KismetMathLibrary.RandomFloatInRange` 0.0 360.0) (`KismetMathLibrary.RandomFloatInRange` 0.0 360.0)) false false))