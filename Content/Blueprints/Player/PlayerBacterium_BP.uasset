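; Player bacterium Blueprint that handles the character's flagella animation and its visual feedback for health, healing and hits.
; Tick drives each flagellum's yaw from a float curve with a different loop period per flagellum and applies a backward force to its bone bodies.
; Health thresholds swap body and flagella materials, and healing spawns an emitter.
; Hits pass to HandleCollision, while GotHitEvent blinks all meshes through a delayed loop during temporary invincibility.
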(event `self.ReceiveTick`
  (params (DeltaSeconds :type "Float (single-precision)"))
  (bind _floatcurve (`self.FloatCurve`))
  (bind (_mintime _maxtime) (`CurveBase.GetTimeRange` _floatcurve))
  (bind _array (`|MakeArray` (`self.FlagelleUp`) (`self.FlagelleLeft`) (`self.FlagelleRight`)))
  (for (_array_element _array_index) _array
    (`SceneComponent.K2_SetRelativeRotation` _array_element (`KismetMathLibrary.MakeRotator` 0.0 0.0 (`CurveFloat.GetFloatValue` _floatcurve (mod (`self.GetGameTimeSinceCreation`) (+ _maxtime (* _maxtime (/ (`KismetMathLibrary.Conv_IntToDouble` _array_index) (`KismetMathLibrary.Conv_IntToDouble` (`KismetArrayLibrary.Array_Length` _array)))))))) false false)
    (`SkeletalMeshComponent.AddForceToAllBodiesBelow` _array_element (-200.0 0.0 0.0) (`SkinnedMeshComponent.GetBoneName` _array_element 1) true true)))

(event `self.HealEffect`
  (`GameplayStatics.SpawnEmitterAtLocation` "/Game/Particles/P_Heal_Blend.P_Heal_Blend" (+ (`SceneComponent.K2_GetComponentLocation` (`self.Bacterium`)) (`KismetMathLibrary.MakeVector` 300.0))))

(event `self.ReceiveHit`
  (params (MyComp :type "PrimitiveComponent Object Reference") (Other :type "Actor Object Reference") (OtherComp :type "PrimitiveComponent Object Reference") (bSelfMoved :type Boolean) (HitLocation :type "Vector Structure") (HitNormal :type "Vector Structure") (NormalImpulse :type "Vector Structure") (Hit :type "HitResult Structure (by ref)"))
  (`self.HandleCollision` MyComp Other OtherComp NormalImpulse Hit))

(event `self.ChangeColor`
  ;[1 1 1] Change Color based on Health
  (`KismetSystemLibrary.Delay` 0.1)
  (if (<= (`self.BacteriumHealth`) 20)
    (`PrimitiveComponent.SetMaterial` (`self.Bacterium`) 0 "/Game/Materials/RedMaterial.RedMaterial")
    (`PrimitiveComponent.SetMaterial` (`self.FlagelleRight`) 0 "/Game/Materials/RedMaterial.RedMaterial")
    (`PrimitiveComponent.SetMaterial` (`self.FlagelleLeft`) 0 "/Game/Materials/RedMaterial.RedMaterial")
    (`PrimitiveComponent.SetMaterial` (`self.FlagelleUp`) 0 "/Game/Materials/RedMaterial.RedMaterial")
    (elif (<= (`self.BacteriumHealth`) 60)
      (`PrimitiveComponent.SetMaterial` (`self.Bacterium`) 0 "/Game/Materials/NiceOrangeMaterial.NiceOrangeMaterial")
      (`PrimitiveComponent.SetMaterial` (`self.FlagelleUp`) 0 "/Game/Materials/NiceOrangeMaterial.NiceOrangeMaterial")
      (`PrimitiveComponent.SetMaterial` (`self.FlagelleRight`) 0 "/Game/Materials/NiceOrangeMaterial.NiceOrangeMaterial")
      (`PrimitiveComponent.SetMaterial` (`self.FlagelleLeft`) 0 "/Game/Materials/NiceOrangeMaterial.NiceOrangeMaterial")
      (else
        (`PrimitiveComponent.SetMaterial` (`self.Bacterium`) 0 null)
        (`PrimitiveComponent.SetMaterial` (`self.FlagelleUp`) 0 null)
        (`PrimitiveComponent.SetMaterial` (`self.FlagelleRight`) 0 null)
        (`PrimitiveComponent.SetMaterial` (`self.FlagelleLeft`) 0 null)))))

(event `self.GotHitEvent`
  (bind _bacterium (`self.Bacterium`))
  (bind _flagelleup (`self.FlagelleUp`))
  (bind _flagelleright (`self.FlagelleRight`))
  (bind _flagelleleft (`self.FlagelleLeft`))
  (`self.SetInvincible` true)
  (set `self.index` 0)
  (if (< (`self.index`) (* (`self.BlinkCount`) 2)) :!label _label
    (`KismetSystemLibrary.Delay` 0.1)
    (`SceneComponent.ToggleVisibility` (`self.Bacterium`) false)
    (`SceneComponent.ToggleVisibility` (`self.FlagelleUp`) false)
    (`SceneComponent.ToggleVisibility` (`self.FlagelleRight`) false)
    (`SceneComponent.ToggleVisibility` (`self.FlagelleLeft`) false)
    (`/Engine/EditorBlueprintResources/StandardMacros.IncrementInt` (`self.index`)
      (:`  `
        (goto _label)))
    (else
      (`self.SetInvincible` false)
      (if (not (`SceneComponent.IsVisible` _bacterium))
        (`SceneComponent.ToggleVisibility` _bacterium false)
        (if (not (`SceneComponent.IsVisible` _flagelleup))
          (`SceneComponent.ToggleVisibility` _flagelleup false))
        (if (not (`SceneComponent.IsVisible` _flagelleright))
          (`SceneComponent.ToggleVisibility` _flagelleright false))
        (if (not (`SceneComponent.IsVisible` _flagelleleft))
          (`SceneComponent.ToggleVisibility` _flagelleleft false))))))

(fn `UserConstructionScript`
  (`self.EnableInput` null))