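; Player virus Blueprint that handles hit and heal feedback for a player made up of single viruses.
; GotHitEvent makes the player invincible and blinks every virus mesh through a delayed loop sized by BlinkCount.
; When the blinking ends, it clears invincibility and re-shows any mesh left hidden.
; HealEffect spawns a heal particle emitter at the player sphere's location.
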(event `self.GotHitEvent`
  (`self.SetInvincible` true)
  (bind _returnvalue (`self.GetSingleViruses`))
  (set `self.index` 0)
  (if (< (`self.index`) (* (`self.BlinkCount`) 2)) :!label _label
    (`KismetSystemLibrary.Delay` 0.1)
    (for _array_element _returnvalue
      (bind _returnvalue_2 (`SingleVirus.GetVirusMeshComponent` _array_element))
      (`/Engine/EditorBlueprintResources/StandardMacros.IsValid` _returnvalue_2
        (:`Is Valid`
          (`SceneComponent.ToggleVisibility` _returnvalue_2 false))))
    (`/Engine/EditorBlueprintResources/StandardMacros.IncrementInt` (`self.index`)
      (:`  `
        (goto _label)))
    (else
      (`self.SetInvincible` false)
      (bind _returnvalue_3 (`self.GetSingleViruses`))
      (for _array_element_2 _returnvalue_3
        (bind _virusmesh (`SingleVirus.VirusMesh` _array_element_2))
        (if (not (`SceneComponent.IsVisible` _virusmesh))
          (`SceneComponent.ToggleVisibility` _virusmesh false))))))

(event `self.HealEffect`
  (`GameplayStatics.SpawnEmitterAtLocation` "/Game/Particles/P_Heal_Blend.P_Heal_Blend" (`SceneComponent.K2_GetComponentLocation` (`self.PlayerSphereComponent`))))

(fn `UserConstructionScript`)