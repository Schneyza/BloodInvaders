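; SingleVirus_BP is one virus body in the player's virus swarm, moved through physics forces on its VirusMesh.
; MovewithFluid passes the mesh to ApplyFluid so the fluid acts on it.
; MovewithPlayer pulls the mesh toward the ParentVirusSwarm actor with a spring-like force that grows with the square of the distance, scaled by PullbackStrength.
; It has no active Tick logic; both moves are custom events.
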(event `self.MoveWithFluid`
  (`FluidDynamics.ApplyFluid` (`self.VirusMesh`)))

(event `self.MoveWithPlayer`
  (bind _virusmesh (`self.VirusMesh`))
  (bind _returnvalue (- (`self.K2_GetActorLocation` (`self.parentVirusSwarm`)) (`SceneComponent.K2_GetComponentLocation` _virusmesh)))
  (`PrimitiveComponent.AddForce` _virusmesh (* _returnvalue (* (`KismetMathLibrary.VSize` _returnvalue) (`self.Pullback Strength`))) "None" false))

(fn `UserConstructionScript`)