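; Dendritic messenger protein actor for Blood Invaders that raises immune cell spawn chances when it escapes the play area along Y.
; Construction gives it a random rotation, and Tick applies force pushing it outward from Y zero toward whichever boundary lies on its side.
; Past either boundary, it calls the game mode to increase B cell and T helper spawn chances and destroys itself.
; Hits are passed to HandleCollision.
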(event `self.ReceiveBeginPlay`)

(event `self.ReceiveTick`
  (params (DeltaSeconds :type "Float (single-precision)"))
  (bind _isoutofbounds (`self.CheckYBoundary`))
  (if _isoutofbounds
    (`self.IncreaseBCellSpawnChance`)
    (`self.IncreaseTHelperSpawnChance`)
    (else
      (`self.Move` DeltaSeconds))))

(event `self.ReceiveHit`
  (params (MyComp :type "PrimitiveComponent Object Reference") (Other :type "Actor Object Reference") (OtherComp :type "PrimitiveComponent Object Reference") (bSelfMoved :type Boolean) (HitLocation :type "Vector Structure") (HitNormal :type "Vector Structure") (NormalImpulse :type "Vector Structure") (Hit :type "HitResult Structure (by ref)"))
  (`self.HandleCollision` MyComp Other OtherComp NormalImpulse Hit))

(event `self.ReceiveDestroyed`)

(fn `CheckYBoundary`
  (returns (IsOutOfBounds :type Boolean))
  (bind _yboundary (`self.YBoundary`))
  (bind _y (.y (`SceneComponent.K2_GetComponentLocation` (`self.Protein1`))))
  (return (or (> _y _yboundary) (< _y (* _yboundary -1.0)))))

(fn `IncreaseBCellSpawnChance`
  (bind _asblood_invaders_game_mode (cast `BloodInvadersGameMode` (`GameplayStatics.GetGameMode`)))
  (`BloodInvadersGameMode.IncreaseBCellSpawnChance` _asblood_invaders_game_mode)
  (`self.K2_DestroyActor`))

(fn `IncreaseTHelperSpawnChance`
  (bind _asblood_invaders_game_mode (cast `BloodInvadersGameMode` (`GameplayStatics.GetGameMode`)))
  (`BloodInvadersGameMode.IncreaseTHelperSpawnChance` _asblood_invaders_game_mode)
  (`self.K2_DestroyActor`))

(fn `Move`
  (params (DeltaSeconds :type "Float (double-precision)"))
  (bind _protein1 (`self.Protein1`))
  (bind _returnvalue (* (`self.MovementSpeed`) DeltaSeconds))
  (if (< (.y (`SceneComponent.K2_GetComponentLocation` (`self.Protein1`))) 0.0)
    (`PrimitiveComponent.AddForce` _protein1 (`KismetMathLibrary.MakeVector` 0.0 (* _returnvalue -1.0)) "None" false)
    (else
      (`PrimitiveComponent.AddForce` _protein1 (`KismetMathLibrary.MakeVector` 0.0 _returnvalue) "None" false))))

(fn `UserConstructionScript`
  (`SceneComponent.K2_SetWorldRotation` (`self.Protein1`) (`KismetMathLibrary.MakeRotator` (`KismetMathLibrary.RandomFloatInRange` 0.0 360.0) (`KismetMathLibrary.RandomFloatInRange` 0.0 360.0) (`KismetMathLibrary.RandomFloatInRange` 0.0 360.0)) false false))