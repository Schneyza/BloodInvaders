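; Protein actor that gets a randomized look and is affected by fluid during play.
; The construction script stores the Protein1 mesh component in Mesh, then gives it a random static mesh and material from the protein arrays and a random world rotation on all three axes.
; Every tick it passes Protein1 to ApplyFluid, whose logic is not defined in this graph.
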(event `self.ReceiveTick`
  (params (DeltaSeconds :type "Float (single-precision)"))
  (`FluidDynamics.ApplyFluid` (`self.Protein1`)))

(fn `UserConstructionScript`
  (bind _protein1 (`self.Protein1`))
  (bind _protein_meshes (`self.Protein Meshes`))
  (bind _protein_materials (`self.Protein Materials`))
  (set `self.Mesh` _protein1)
  (`StaticMeshComponent.SetStaticMesh` _protein1 (`|GetArrayItem` _protein_meshes (`KismetMathLibrary.RandomInteger` (`KismetArrayLibrary.Array_Length` _protein_meshes))))
  (`PrimitiveComponent.SetMaterial` _protein1 0 (`|GetArrayItem` _protein_materials (`KismetMathLibrary.RandomInteger` (`KismetArrayLibrary.Array_Length` _protein_materials))))
  (`SceneComponent.K2_SetWorldRotation` _protein1 (`KismetMathLibrary.MakeRotator` (`KismetMathLibrary.RandomFloatInRange` 0.0 360.0) (`KismetMathLibrary.RandomFloatInRange` 0.0 360.0) (`KismetMathLibrary.RandomFloatInRange` 0.0 360.0)) false false))