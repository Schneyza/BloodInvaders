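; Score actor that tracks per-entry counts and turns them into weighted scores.
; Parallel maps hold each entry's name, count and multiplier, with lookups falling back to defaults for missing keys.
; IncrementEntry bumps a count and prints a debug string, while getters derive count-times-multiplier scores, bundle an entry's details, and total scores across all named entries.
; The event graph and construction script are empty.
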(fn `Get Complete Score`
  (params (NewParam :type "/Game/Blueprints/EScoreEntry Enum" :default "NewEnumerator4"))
  (returns (Name :type Text) (count :type Integer) (Mult :type Integer) (Score :type Integer))
  (bind (_name _count _mult _score) (`self.Get Complete Score M` NewParam))
  (return _name _count _mult _score))

(fn `Get Entries`
  (returns (`Return Value` :type "Array of /Game/Blueprints/EScoreEntry Enum"))
  (bind _keys (`BlueprintMapLibrary.Map_Keys` (`self.Name Dict`)))
  (return _keys))

(fn `Get Total Score`
  (returns (`Return Value` :type Integer))
  (locals (Score :type Integer :default 0))
  (bind _return_value (`self.Get Entries`))
  (for _array_element _return_value
    (set `local.Score` (+ (`local.Score`) (`self.Get Score` _array_element))))
  (return (`local.Score`)))

(fn `Increment Entry`
  (params (Entry :type "/Game/Blueprints/EScoreEntry Enum" :default "NewEnumerator4"))
  (bind (_value _returnvalue) (`BlueprintMapLibrary.Map_Find` (`self.Count Dict`) Entry))
  (`BlueprintMapLibrary.Map_Add` (`self.Count Dict`) Entry (+ (`KismetMathLibrary.SelectInt` _value 0 _returnvalue) 1))
  (`KismetSystemLibrary.PrintString` "Hello"))

(fn `UserConstructionScript`)