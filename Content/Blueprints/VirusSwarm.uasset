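; VirusSwarm is an actor that holds a cluster of five SingleVirus actors loosely around its Sphere component.
; The construction script adds them as child actors at random local offsets and stores them in Viruses.
; Each Tick pushes every virus's Object toward the Sphere with a force that grows with the square of its distance, scaled by PullbackStrength, acting as a nonlinear spring.
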(event `self.ReceiveTick`
  (params (DeltaSeconds :type "Float (single-precision)"))
  (for _array_element (`self.Viruses`)
    (bind _object (`/Game/Blueprints/SingleVirus.Object` _array_element))
    (bind _returnvalue (- (`SceneComponent.K2_GetComponentLocation` (`self.Sphere`)) (`SceneComponent.K2_GetComponentLocation` _object)))
    (`PrimitiveComponent.AddForce` _object (* _returnvalue (* (`KismetMathLibrary.VSize` _returnvalue) (`self.Pullback strength`))) "None" false)))

(fn `UserConstructionScript`
  (for _ (range 1 6)
    (bind _returnvalue (`AddComponent|NODE_AddChildActorComponent-2` :`RelativeTransform` (`KismetMathLibrary.Conv_VectorToTransform` (`KismetMathLibrary.MakeVector` (`KismetMathLibrary.RandomFloatInRange` 0.0 100.0) (`KismetMathLibrary.RandomFloatInRange` 0.0 100.0) (`KismetMathLibrary.RandomFloatInRange` 0.0 100.0)))))
    (bind _assingle_virus (cast `/Game/Blueprints/SingleVirus` (`ChildActorComponent.ChildActor` _returnvalue)))
    (`KismetArrayLibrary.Array_Add` (`self.Viruses`) _assingle_virus)))