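; Spawn area Blueprint that repeatedly adds child actors, counted by NumNeutros, at random points within a box sized from AreaExtents at construction.
; The spawn loop runs at BeginPlay, then re-runs from Tick through a random 2–5 second Delay, adding a second actor per iteration after 15 seconds of game time.
; Positions come from a random stream on a flat plane.
; The SpawnSetting switch and NumMacros loop are unconnected.
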(event `self.ReceiveBeginPlay`
  (bind _stream (`self.Stream`))
  (bind (_boxextent_x _boxextent_y) (`KismetMathLibrary.BreakVector` (`BoxComponent.BoxExtent` (`self.SpawnArea`))))
  (bind _returnvalue (`KismetMathLibrary.MakeVector` (`KismetMathLibrary.RandomFloatInRangeFromStream` (* _boxextent_x -1.0) _boxextent_x _stream) (`KismetMathLibrary.RandomFloatInRangeFromStream` (* _boxextent_y -1.0) _boxextent_y _stream)))
  (for _ (range (+ (`self.NumNeutros`) 1)) :!label _label
    (`AddComponent|NODE_AddChildActorComponent-4` :`RelativeTransform` (`KismetMathLibrary.MakeTransform` _returnvalue))
    (if (>= (`KismetMathLibrary.FTrunc` (`KismetSystemLibrary.GetGameTimeInSeconds`)) 15)
      (`AddComponent|NODE_AddChildActorComponent-6` :`RelativeTransform` (`KismetMathLibrary.MakeTransform` _returnvalue)))))

(event `self.ReceiveTick`
  (params (DeltaSeconds :type "Float (single-precision)"))
  (`KismetSystemLibrary.Delay` (`KismetMathLibrary.Conv_IntToDouble` (`KismetMathLibrary.RandomIntegerInRange` 2 5)))
  (goto _label))

(fn `UserConstructionScript`
  (`BoxComponent.SetBoxExtent` (`self.SpawnArea`) (`self.AreaExtents`) true))