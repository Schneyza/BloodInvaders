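; BacteriumNew_BP is a bacterium actor that procedurally animates its three flagella (up, left, right).
; Each Tick sets every flagellum's relative yaw from a float curve sampled on looping game time, with a longer loop per index so they drift out of sync.
; It also applies a constant negative-X acceleration to the physics bodies below bone index 1, so each flagellum trails through physics simulation.
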(event `self.ReceiveTick`
  (params (DeltaSeconds :type "Float (single-precision)"))
  (bind _floatcurve (`self.FloatCurve`))
  (bind (_mintime _maxtime) (`CurveBase.GetTimeRange` _floatcurve))
  (bind _array (`|MakeArray` (`self.FlagelleUp`) (`self.FlagelleLeft`) (`self.FlagelleRight`)))
  (for (_array_element _array_index) _array
    (`SceneComponent.K2_SetRelativeRotation` _array_element (`KismetMathLibrary.MakeRotator` 0.0 0.0 (`CurveFloat.GetFloatValue` _floatcurve (mod (`self.GetGameTimeSinceCreation`) (+ _maxtime (* _maxtime (/ (`KismetMathLibrary.Conv_IntToDouble` _array_index) (`KismetMathLibrary.Conv_IntToDouble` (`KismetArrayLibrary.Array_Length` _array)))))))) false false)
    (`SkeletalMeshComponent.AddForceToAllBodiesBelow` _array_element (-200.0 0.0 0.0) (`SkinnedMeshComponent.GetBoneName` _array_element 1) true true)))

(fn `UserConstructionScript`)