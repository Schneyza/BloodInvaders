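; Macrophage actor with a morphing body and physics-driven pseudopodia that reach toward a grab target.
; The construction script spawns a ring of skeletal mesh pseudopodia, each with a randomized speed.
; Each tick layers two morph target sets on the body at different rates.
; It also applies velocity impulses to each pseudopod's second-to-last bone toward GrabTarget, stopping once the End socket is close enough.
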(event `UpdatePseudopodia`
  (for _array_element (`self.Pseudopodias`)
    (bind _impulsedir (`self.Close Enough` (- (`self.GrabTarget`) (`SceneComponent.GetSocketLocation` (break `/Game/Models/MacrophageNew/PseudopodiaInfo` _array_element) "End"))))
    (`PrimitiveComponent.AddImpulse` (break `/Game/Models/MacrophageNew/PseudopodiaInfo` _array_element) (* _impulsedir (`.speed_8_EAF28D134B542D6945F57D9435D24876` (break `/Game/Models/MacrophageNew/PseudopodiaInfo` _array_element))) (`SkinnedMeshComponent.GetBoneName` (break `/Game/Models/MacrophageNew/PseudopodiaInfo` _array_element) (- (`SkinnedMeshComponent.GetNumBones` (break `/Game/Models/MacrophageNew/PseudopodiaInfo` _array_element)) 2)) true)))

(event `UpdateMorph`
  (`/Game/Models/MacrophageNew/MorphLib.MorphTarget` (`self.MacrophageBody`) (* (`self.GetGameTimeSinceCreation`) 0.3) (`self.Morph Names Big`))
  (`/Game/Models/MacrophageNew/MorphLib.MorphTarget` (`self.MacrophageBody`) (* (`self.GetGameTimeSinceCreation`) 0.7) (`self.Morph Names Small`)))

(event `self.ReceiveTick`
  (params (DeltaSeconds :type "Float (single-precision)"))
  (`self.UpdateMorph`)
  (`self.UpdatePseudopodia`))

(fn `Close Enough`
  (params (RelativTarget :type "Vector Structure"))
  (returns (ImpulseDir :type "Vector Structure"))
  (if (<= (`KismetMathLibrary.VSize` RelativTarget) (`self.Pseudopodia Close Enough`))
    (return (0.0 0.0 0.0))
    (else
      (return (`KismetMathLibrary.Normal` RelativTarget)))))

(fn `Limit Distance`
  (params (Target :type "Vector Structure") (Source :type "Vector Structure") (`Max Distance` :type "Float (double-precision)") (`Min Distance` :type "Float (double-precision)"))
  (returns (`Limited Target` :type "Vector Structure"))
  (bind _returnvalue (- Target Source))
  (bind _max_distance (`local.Max Distance`))
  (bind _min_distance (`local.Min Distance`))
  (bind _returnvalue_2 (`KismetMathLibrary.VSize` _returnvalue))
  (bind _returnvalue_3 (`KismetMathLibrary.Normal` _returnvalue))
  (if (<= _returnvalue_2 _max_distance)
    (if (>= _returnvalue_2 _min_distance)
      (return (0.0 0.0 0.0))
      (else
        (return (* _returnvalue_3 _min_distance))))
    (else
      (return (* _returnvalue_3 _max_distance)))))

(fn `UserConstructionScript`
  (bind _returnvalue_location (`KismetMathLibrary.BreakTransform` (`self.GetTransform`)))
  (bind _pseudopodia_count (`self.Pseudopodia Count`))
  (bind _pseudopodia_spawn_radius (`self.Pseudopodia Spawn Radius`))
  (for _index (range 1 (+ _pseudopodia_count 1))
    (bind _returnvalue (* 360.0 (/ (`KismetMathLibrary.Conv_IntToDouble` _index) (`KismetMathLibrary.Conv_IntToDouble` _pseudopodia_count))))
    (bind _returnvalue_2 (`AddComponent|NODE_AddSkeletalMeshComponent-1` :`RelativeTransform` (`KismetMathLibrary.MakeTransform` (+ (`KismetMathLibrary.MakeVector` (* (`KismetMathLibrary.DegSin` _returnvalue) _pseudopodia_spawn_radius) (* _pseudopodia_spawn_radius (`KismetMathLibrary.DegCos` _returnvalue))) (0.0 0.0 0.0) _returnvalue_location) (struct :`Pitch` 90.0))))
    (`KismetArrayLibrary.Array_Add` (`self.Pseudopodias`) (make `/Game/Models/MacrophageNew/PseudopodiaInfo` _returnvalue_2 (* (`self.Pseudopodia Speed`) (`KismetMathLibrary.RandomFloatInRange` 0.5 2.0))))))