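; Actor Blueprint that continuously animates a neutrophil mesh by cycling through its morph targets in a loop.
; Each Tick maps time since creation, at half speed, onto a wrapping index into the MorphNames array.
; The fractional part linearly crossfades the current morph target out and the next one in, wrapping back to the first after the last.
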(event `self.ReceiveTick`
  (params (DeltaSeconds :type "Float (single-precision)"))
  (bind _returnvalue (mod (* (`self.GetGameTimeSinceCreation`) 0.5) (`KismetMathLibrary.Conv_IntToDouble` (`KismetArrayLibrary.Array_Length` (`self.morphNames`)))))
  (bind _returnvalue_2 (`KismetMathLibrary.FTrunc` _returnvalue))
  (bind _returnvalue_3 (- _returnvalue (`KismetMathLibrary.Conv_IntToDouble` _returnvalue_2)))
  (`SkeletalMeshComponent.SetMorphTarget` (`self.Neutrophil`) (`|GetArrayItem` (`self.morphNames`) _returnvalue_2) (- 1.0 _returnvalue_3) true)
  (`SkeletalMeshComponent.SetMorphTarget` (`self.Neutrophil`) (`|GetArrayItem` (`self.morphNames`) (mod (+ _returnvalue_2 1) (`KismetArrayLibrary.Array_Length` (`self.morphNames`)))) _returnvalue_3 true))

(event `self.ReceiveBeginPlay`)

(fn `UserConstructionScript`)